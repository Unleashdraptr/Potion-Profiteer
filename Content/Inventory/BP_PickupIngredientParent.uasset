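; Parent Blueprint for world ingredient pickups that hand their item data to whoever collects them.
; On overlap with a BPI_PickupIngredient implementer that is not another pickup, it sends class, icon, stack size, name, description and tier, then destroys itself.
; PushPickupIngredientAway applies a velocity-change impulse to the PaperSprite along the player camera's forward direction.
; GetPickupIngredientData is a stub returning empty values.
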(event `self.ReceiveActorBeginOverlap`
  (params (OtherActor :type "Actor Object Reference"))
  (if (`KismetSystemLibrary.DoesImplementInterface` OtherActor "/Game/Inventory/BPI_PickupIngredient.BPI_PickupIngredient_C")
    (if (not (`KismetMathLibrary.ClassIsChildOf` (`GameplayStatics.GetObjectClass` OtherActor) "BP_PickupIngredientParent_C"))
      (message `/Game/Inventory/BPI_PickupIngredient.PickupIngredient` OtherActor (`self.IngredientClass`) (`self.IngredientIcon`) (`self.IngredientStackSize`) (`self.IngredientName`) (`self.IngredientDescription`) (`self.IngredientTier`))
      (`self.K2_DestroyActor`))))

(event `/Game/Inventory/BPI_PickupIngredient.PushPickupIngredientAway`
  (bind _returnvalue (`KismetMathLibrary.GetForwardVector` (`PlayerCameraManager.GetCameraRotation` (`GameplayStatics.GetPlayerCameraManager` 0))))
  (`PrimitiveComponent.AddVelocityChangeImpulseAtLocation` (`self.PaperSprite`) (* _returnvalue 250.0) (+ (`self.K2_GetActorLocation`) (* _returnvalue (15.0 0.0 0.0))) "None"))

(fn `GetPickupIngredientData`
  (returns (IngredientClass :type "Actor Class Reference") (CurrentStackAmount :type Integer) (MaxStackAmount :type Integer) (IngredientName :type String) (IngredientDescription :type String) (IngredientTier :type String))
  (return null 0 0 "" "" ""))

(fn `UserConstructionScript`)