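; BP_Crop is a crop actor that serves as the entry point to the harvesting minigame.
; Its TextRender starts hidden and is shown only while something overlaps the TriggerZone, with no filter on the overlapping actor.
; The Talk event creates the HarvestingMinigameUI widget for the first player, adds it to the viewport, and removes HarvestingMinigameStarterUpper widgets from their parent.
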(event `self.TriggerZone.OnComponentBeginOverlap`
  (params (OverlappedComponent :type "PrimitiveComponent Object Reference") (OtherActor :type "Actor Object Reference") (OtherComp :type "PrimitiveComponent Object Reference") (OtherBodyIndex :type Integer) (bFromSweep :type Boolean) (SweepResult :type "HitResult Structure (by ref)"))
  (`SceneComponent.SetVisibility` (`self.TextRender`) true false))

(event `self.TriggerZone.OnComponentEndOverlap`
  (params (OverlappedComponent :type "PrimitiveComponent Object Reference") (OtherActor :type "Actor Object Reference") (OtherComp :type "PrimitiveComponent Object Reference") (OtherBodyIndex :type Integer))
  (`SceneComponent.SetVisibility` (`self.TextRender`) false false))

(event `self.ReceiveBeginPlay`
  (`SceneComponent.SetVisibility` (`self.TextRender`) false false))

(event `/Game/Dialogue/BPI_Dialogue.Talk`
  (bind _returnvalue (`|CreateWidget` "/Game/Harvesting/HarvestingMinigameUI.HarvestingMinigameUI_C" (`GameplayStatics.GetPlayerController` 0)))
  (`UserWidget.AddToViewport` _returnvalue 0)
  (bind _foundwidgets (`WidgetBlueprintLibrary.GetAllWidgetsOfClass` "/Game/Harvesting/HarvestingMinigameStarterUpper.HarvestingMinigameStarterUpper_C" false))
  (`Widget.RemoveFromParent` _foundwidgets))

(fn `UserConstructionScript`)